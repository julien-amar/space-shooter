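; Projectile actor that flies along its local axes at a set Speed and damages what it hits.
; The construction script creates a dynamic material on the Projectile component, tinted with ProjectileColor at BeginPlay.
; Tick moves it by unswept local offsets, so hits come from overlap events.
; Overlaps ignore the owner and BPProjectileLaser actors; others receive fixed DMGShot damage, and the projectile spawns a pixel explosion and destroys itself.
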(event `self.ReceiveBeginPlay`
  ;[1 1 1] Set Material with Color
  (`MaterialInstanceDynamic.SetVectorParameterValue` (`self.ProjectileMaterial`) "Color2" (`self.ProjectileColor`)))

(event `self.ReceiveTick`
  (params (DeltaSeconds :type "Float (single-precision)"))
  ;[1 1 1] Move Projectile
  (`self.K2_AddActorLocalOffset` (* (`self.Speed`) DeltaSeconds)))

(event `self.Projectile.OnComponentBeginOverlap`
  (params (OtherActor :type "Actor Object Reference") (OtherComp :type "PrimitiveComponent Object Reference") (OtherBodyIndex :type Integer) (bFromSweep :type Boolean) (SweepResult :type "HitResult Structure (by ref)"))
  ;[1 1 1] Collision events
  (if (!= OtherActor (`self.ProjectileOwner`))
    (cast `/Game/Blueprints/BPProjectileLaser` OtherActor
      (:`CastFailed`
        (if (not false)
          (`GameplayStatics.ApplyDamage` OtherActor 20.0 null null "/Game/Blueprints/DMGShot.DMGShot_C")
          (`GameplayStatics.SpawnEmitterAtLocation` "/Game/Art/Particles/P_Pixel_Explosion.P_Pixel_Explosion" (`self.K2_GetActorLocation`))
          (`self.K2_DestroyActor`))))))

(fn `UserConstructionScript`
  (bind _returnvalue (`PrimitiveComponent.CreateDynamicMaterialInstance` (`self.Projectile`) 0 null))
  (set `self.ProjectileMaterial` _returnvalue))