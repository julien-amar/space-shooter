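; Enemy actor that drops in with a spawn animation, then patrols at a random speed and initial direction, reversing when it hits a non-pawn.
; A randomized Delay on Tick paces projectile fire along Z whenever the player is close on the X axis.
; Ramming a pawn deals collision damage and destroys the enemy, as does losing all health, with both paths awarding score through BPGameController.
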(event `self.ReceiveBeginPlay`
  (bind _spawnlocation (`self.SpawnLocation`))
  (bind _returnvalue (+ (`self.Yaw`) 0.0))
  ;[1 1 1] Movement Randomizer
  (set `self.Yaw` (+ (.yaw (`self.K2_GetActorRotation` (`self.GetInstigator`))) 1.0))
  (set `self.MoveDirection` (`KismetMathLibrary.RandomBool`))
  (set `self.MoveSpeed` (`KismetMathLibrary.RandomFloatInRange` (`self.MinimumMoveSpeed`) (`self.MaximumMoveSpeed`)))
  ;[1 1 1] Spawn Animation
  (set `self.SpawnLocation` (`self.K2_GetActorLocation`))
  (bind (_direction _plop) (`Timeline|SpawnAnimation`)
    (:`Update`
      (`self.K2_SetActorLocation` (`KismetMathLibrary.VLerp` _spawnlocation (- _spawnlocation (0.0 0.0 60.0)) _plop))
      (`self.SetActorRotation` (`KismetMathLibrary.RLerp` (`KismetMathLibrary.MakeRotator` 0.0 0.0 _returnvalue) (`KismetMathLibrary.MakeRotator` 0.0 0.0 _returnvalue) _plop)))
    (:`Finished`
      (set `self.MoveEnabled` true))))

(event `self.ReceiveTick`
  (params (DeltaSeconds :type "Float (single-precision)"))
  (bind _returnvalue (`GameplayStatics.GetPlayerPawn` 0))
  ;[1 1 1] Movement
  (if (`self.MoveEnabled`)
    (`self.K2_SetActorLocation` (+ (`self.K2_GetActorLocation`) (* (`KismetMathLibrary.GreaterGreater_VectorRotator` (`KismetMathLibrary.MakeVector` (* (`self.MoveSpeed`) (`KismetMathLibrary.SelectFloat` 1.0 -1.0 (`self.MoveDirection`)))) (`KismetMathLibrary.MakeRotator` 0.0 0.0 (`self.Yaw`))) DeltaSeconds)) true)
    ;[1 1 1] Fire
    (`/Engine/EditorBlueprintResources/StandardMacros.IsValid` _returnvalue
      (:`Is Valid`
        (`KismetSystemLibrary.Delay` (`KismetMathLibrary.RandomFloatInRange` 0.1 0.4))
        (if (<= (`KismetMathLibrary.VSize` (* (- (`self.K2_GetActorLocation` _returnvalue) (`self.K2_GetActorLocation`)) (1.0 0.0 0.0))) 120.0)
          (`|SpawnActorFromClass` "/Game/Blueprints/BPProjectileEnemy.BPProjectileEnemy_C" (`self.GetTransform`) "Undefined" "OverrideRootScale" null (`KismetMathLibrary.MakeColor` 1.0 0.3 0.05) (`KismetMathLibrary.MakeVector` 0.0 0.0 (`self.AttackSpeed`)) self)
          (`GameplayStatics.PlaySoundAtLocation` "/Game/Audio/EnemyShot.EnemyShot" (`self.K2_GetActorLocation`)))))))

(event `self.ReceiveHit`
  (params (MyComp :type "PrimitiveComponent Object Reference") (Other :type "Actor Object Reference") (OtherComp :type "PrimitiveComponent Object Reference") (bSelfMoved :type Boolean) (HitLocation :type "Vector Structure") (HitNormal :type "Vector Structure") (NormalImpulse :type "Vector Structure") (Hit :type "HitResult Structure (by ref)"))
  ;[1 1 1] Death
  (bind _aspawn (cast `Pawn` Other)
    (:`then`
      (`GameplayStatics.ApplyDamage` _aspawn 10.0 null null "/Game/Blueprints/DMGCollision.DMGCollision_C")
      (bind _outactors (`GameplayStatics.GetAllActorsOfClass` "/Game/Blueprints/BPGameController.BPGameController_C" :!label _label))
      (`/Game/Blueprints/BPGameController.ScoreEvent` (`KismetArrayLibrary.Array_Get` _outactors) 20)
      (`self.K2_DestroyActor`))
    (:`CastFailed`
      ;[1 1 1] Colision
      (set `self.MoveDirection` (not (`self.MoveDirection`))))))

(event `self.ReceiveAnyDamage`
  (params (Damage :type "Float (single-precision)") (DamageType :type "DamageType Object Reference") (InstigatedBy :type "Controller Object Reference") (DamageCauser :type "Actor Object Reference"))
  ;[1 1 1] Death
  (set `self.Health` (`KismetMathLibrary.FClamp` (- (`self.Health`) Damage) 0.0 100.0))
  (if (<= (`self.Health`) 0.0)
    (`GameplayStatics.SpawnEmitterAtLocation` "/Game/Art/Particles/P_Pixel_Explosion_Enemy.P_Pixel_Explosion_Enemy" (`self.K2_GetActorLocation`))
    (goto _label)))

(fn `UserConstructionScript`)