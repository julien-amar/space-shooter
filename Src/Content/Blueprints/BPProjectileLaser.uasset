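; Laser projectile actor that snaps onto its owner and plays as an extending beam rather than using a movement component.
; Construction script creates a dynamic material on the projectile mesh, which BeginPlay tints with the projectile color.
; A Movement timeline drives the mesh's scale and relative location, then destroys the actor when finished.
; Overlapping any actor other than the owner applies fixed shot-type damage.
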(event `self.ReceiveBeginPlay`
  ;[1 1 1] Set Material with Color
  (`self.K2_AttachRootComponentToActor` (`self.ProjectileOwner`) "None" "SnapToTarget")
  (`MaterialInstanceDynamic.SetVectorParameterValue` (`self.ProjectileMaterial`) "Color2" (`self.ProjectileColor`))
  (bind (_direction _extend _move) (`Timeline|Movement`)
    (:`Update`
      (`SceneComponent.SetWorldScale3D` (`self.Projectile`) _extend)
      (`SceneComponent.K2_SetRelativeLocation` (`self.Projectile`) _move false false))
    (:`Finished`
      (`self.K2_DestroyActor`))))

(event `self.Projectile.OnComponentBeginOverlap`
  (params (OtherActor :type "Actor Object Reference") (OtherComp :type "PrimitiveComponent Object Reference") (OtherBodyIndex :type Integer) (bFromSweep :type Boolean) (SweepResult :type "HitResult Structure (by ref)"))
  ;[1 1 1] Collision events
  (if (!= OtherActor (`self.ProjectileOwner`))
    (`GameplayStatics.ApplyDamage` OtherActor 150.0 null null "/Game/Blueprints/DMGShot.DMGShot_C")))

(fn `UserConstructionScript`
  (bind _returnvalue (`PrimitiveComponent.CreateDynamicMaterialInstance` (`self.Projectile`) 0 null))
  (set `self.ProjectileMaterial` _returnvalue))