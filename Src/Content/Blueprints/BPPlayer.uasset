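; Player actor that flies on a plane set by its spawn yaw and fires two weapon types.
; A spawn timeline lifts and spins it into place, then enables movement.
; Tick eases horizontal and vertical speeds toward input, moves along local X and Z, and turns yaw with horizontal speed.
; Held primary fire repeats twin projectiles from Left and Right on a looping timer, while secondary fire spawns a laser gated by a timeline cooldown.
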(event Custom|FireReset
  ;[1 1 1] Primary Fire
  (CallFunction|PrimaryFire (Variables|Default|GetLeft))
  (CallFunction|PrimaryFire (Variables|Default|GetRight)))

(event EventBeginPlay
  ;[1 1 1] Play Spawn Animation
  (Variables|Default|SetYaw (.Yaw (Math|Rotator|BreakRotator (Transformation|GetActorRotation (Game|GetInstigator)))))
  (Variables|Default|SetSpawnLocation (Transformation|GetActorLocation))
  (bind _lerp (Timeline|SpawnAnimation Play)
    (:Update
      (Transformation|SetActorLocation (Math|Vector|Lerp(Vector) (Variables|Default|GetSpawnLocation) (+ (Variables|Default|GetSpawnLocation) "0, 0,60.000000") _lerp) false false)
      (Transformation|SetActorRotation (Math|Rotator|Lerp(Rotator) "0, 0, 0" (Math|Rotator|MakeRotator 0.0 0.0 (+ 7.2e+02 (Variables|Default|GetYaw))) _lerp)))
    (:Finished
      (Variables|Default|SetbMovementEnabled true))))

(event EventTick
  (params (DeltaSeconds :type Float%20%28single-precision%29))
  ;[1 1 1] PlayerMovement
  (Variables|Default|SetDeltaSeconds DeltaSeconds)
  (if (Variables|Default|GetbMovementEnabled)
    (bind _return_direction (CallFunction|Movement (Variables|Default|GetHozSpeed) (Input|AxisValues|GetMoveRight)))
    (Variables|Default|SetHozSpeed _return_direction)
    (bind _return_direction_2 (CallFunction|Movement (Variables|Default|GetVertSpeed) (Input|AxisValues|GetMoveForward)))
    (Variables|Default|SetVertSpeed _return_direction_2)
    (Transformation|SetActorLocation (+ (Transformation|GetActorLocation) (Math|Vector|RotateVector (Math|Vector|MakeVector (stale _output_get) 0.0 (stale _output_get)) (Math|Rotator|MakeRotator 0.0 0.0 (Variables|Default|GetYaw)))) false false)
    (Transformation|SetActorRotation (Math|Interpolation|RInterpTo (Transformation|GetActorRotation) (Math|Rotator|MakeRotator 0.0 0.0 (+ (* (Variables|Default|GetHozSpeed) -1e+01) (Variables|Default|GetYaw))) (Variables|Default|GetDeltaSeconds) 0.0))))

(event Input|ActionEvents|InputActionPrimaryFire
  (params (Key :type Key%20Structure :default "AnyKey"))
  ;[1 1 1] Primary Fire
  (:Pressed
    (bind _returnvalue (Utilities|Time|SetTimerbyFunctionName 0 "FireReset" 0.2 true))
    (Variables|Default|SetTimeHandle _returnvalue)
    (CallFunction|PrimaryFire (Variables|Default|GetLeft))
    (CallFunction|PrimaryFire (Variables|Default|GetRight)))
  (:Released
    (Class|KismetSystemLibrary|ClearTimerHandle (Variables|Default|GetTimeHandle))))

(event Input|ActionEvents|InputActionSecondlyFire
  (params (Key :type Key%20Structure :default "AnyKey"))
  ;[1 1 1] Fire Laser
  (:Pressed
    (if (Variables|Default|GetbLaserReady)
      (Variables|Default|SetbLaserReady false)
      (Game|SpawnActorfromClass "/Game/Blueprints/BPProjectileLaser.BPProjectileLaser_C" (Transformation|GetActorTransform) "Undefined" 0 (Math|Color|MakeColor 0.2 0.2 1.0 1.0) self)
      (Timeline|LaserLifeTime Play
        (:Finished
          (Variables|Default|SetbLaserReady true))))))

(fn ConstructionScript)

(fn Movement
  (params (Speed :type Float%20%28single-precision%29) (Direction :type Float%20%28single-precision%29))
  (bind _output_get (Variables|Default|SetCurrentSpeed (Math|Interpolation|FInterpTo Speed (* (* Direction (Variables|Default|GetMovementSpeed)) (Variables|Default|GetDeltaSeconds)) (Variables|Default|GetDeltaSeconds) 4.0)))
  (return _output_get))

(fn PrimaryFire
  (params (Location :type Scene%20Component%20Object%20Reference))
  (Game|SpawnActorfromClass "/Game/Blueprints/BPProjectile.BPProjectile_C" (Transformation|GetWorldTransform Location) "Undefined" 0 (Math|Color|MakeColor 0.6 0.3 0.6 1.0) (Math|Vector|MakeVector 0.0 0.0 7e+02) self))