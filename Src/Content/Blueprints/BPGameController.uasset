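; Game controller actor for a ship game that runs the play loop, spawning and possessing the player while acting as the camera view.
; A gated Tick with random Delay spawns random enemies along a horizontal offset, lengthening the clamped interval each spawn.
; Destroy bindings shake the camera on deaths, play enemy explosions, and clear enemies and restart when the player dies, unless QuitGame closes that gate.
; A trigger destroys off-screen enemies.
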(event `self.ReceiveTick`
  (params (DeltaSeconds :type "Float (single-precision)"))
  (bind _spawninterval (`self.SpawnInterval`))
  (bind _enemyspawnpoint (`self.EnemySpawnPoint`))
  (bind _maxspawnhozoffset (`self.MaxSpawnHozOffset`))
  (bind _actorarray (`self.ActorArray`))
  ;[1 1 1] Spawn Enemies at random locations
  (`/Engine/EditorBlueprintResources/StandardMacros.Gate` true :!label _label
    (:`Exit`
      (`KismetSystemLibrary.Delay` (`KismetMathLibrary.RandomFloatInRange` _spawninterval (+ _spawninterval 0.1)))
      (bind _returnvalue (`|SpawnActorFromClass` (`KismetArrayLibrary.Array_Get` _actorarray (`KismetMathLibrary.RandomInteger` (`KismetArrayLibrary.Array_Length` _actorarray))) (`KismetMathLibrary.MakeTransform` (+ (`SceneComponent.K2_GetComponentLocation` _enemyspawnpoint) (`KismetMathLibrary.LessLess_VectorRotator` (`KismetMathLibrary.MakeVector` 0.0 (`KismetMathLibrary.RandomFloatInRange` (* _maxspawnhozoffset -1.0) _maxspawnhozoffset)) (`self.K2_GetActorRotation`))) (`SceneComponent.K2_GetComponentRotation` _enemyspawnpoint) (1.0 1.0 1.0)) "Undefined" "OverrideRootScale"))
      (`KismetArrayLibrary.Array_Add` (`self.SpawnedEnemies`) _returnvalue)
      (add `self.OnDestroyed` _returnvalue (delegate `EnemyDestroyed`))
      (set `self.SpawnInterval` (`KismetMathLibrary.FClamp` (+ (`self.SpawnInterval`) 0.3) 0.7 10.0)))))

(event `self.ReceiveBeginPlay`
  ;[1 1 1] Controlling the start and end of game
  (`self.StartGame`))

(event `ResetSpawnEnemies`
  ;[1 1 1] Spawn Enemies at random locations
  (goto _label :!via `Open`))

(event `StopSpawningEnemies`
  (bind _spawnedenemies (`self.SpawnedEnemies`))
  ;[1 1 1] Spawn Enemies at random locations
  (for _array_element _spawnedenemies
    (`self.K2_DestroyActor` _array_element))
  (`KismetArrayLibrary.Array_Clear` _spawnedenemies)
  (goto _label :!via `Close`))

(event `StartGame`
  (bind _playership (`self.PlayerShip`))
  ;[1 1 1] Controlling the start and end of game
  (set `self.bPlayerDead` false)
  (`AudioComponent.Play` (`self.Action`) 0.0)
  (`|ExecutionSequence`
    (:`then_0`
      (set `self.SpawnInterval` 1.0)
      (`self.ResetSpawnEnemies`)
      (bind _returnvalue (`|SpawnActorFromClass` "/Game/Blueprints/BPPlayer.BPPlayer_C" (`SceneComponent.K2_GetComponentToWorld` (`self.PlayerSpawnPoint`)) "Undefined" "OverrideRootScale"))
      (set `self.PlayerShip` _returnvalue)
      (`Controller.Possess` (`GameplayStatics.GetPlayerController` 0) _playership)
      (add `self.OnDestroyed` _playership (delegate `PlayerKilled`))
      (`PlayerController.SetViewTargetWithBlend` (`GameplayStatics.GetPlayerController` 0) self 0.0 "VTBlend_Linear" 0.0 true))
    (:`then_1`
      (goto _label_2 :!via `Open`))))

(event `PlayerKilled`
  ;[1 1 1] Controlling the start and end of game
  (set `self.bPlayerDead` true)
  (`self.StopSpawningEnemies`)
  (`PlayerController.SetViewTargetWithBlend` (`GameplayStatics.GetPlayerController` 0) self 0.0 "VTBlend_Linear" 0.0 false)
  (`/Engine/EditorBlueprintResources/StandardMacros.Gate` true :!label _label_2
    (:`Exit`
      (`self.StartGame`))))

(event `EnemyDestroyed`
  ;[1 1 1] Spawn Enemies at random locations
  (if (not (`self.bPlayerDead`))
    (`self.PlayCameraShake`)
    (`/Engine/EditorBlueprintResources/StandardMacros.DoOnce` false :!label _label_3
      (:`Completed`
        (`GameplayStatics.PlaySoundAtLocation` "/Game/Audio/Explosion.Explosion")
        (goto _label_3 :!via `Reset`)))))

(event `QuitGame`
  ;[1 1 1] Controlling the start and end of game
  (`|ExecutionSequence`
    (:`then_0`
      (goto _label_2 :!via `Close`))
    (:`then_1`
      (`self.K2_DestroyActor` (`self.PlayerShip`))
      (`self.PlayCameraShake`)
      (`AudioComponent.Stop` (`self.Action`)))))

(event `self.Trigger.OnComponentBeginOverlap`
  (params (OtherActor :type "Actor Object Reference") (OtherComp :type "PrimitiveComponent Object Reference") (OtherBodyIndex :type Integer) (bFromSweep :type Boolean) (SweepResult :type "HitResult Structure (by ref)"))
  ;[1 1 1] Destroy off screen objects
  (if (`KismetArrayLibrary.Array_Contains` (`self.SpawnedEnemies`) OtherActor)
    (`self.K2_DestroyActor` OtherActor)))

(event `PlayCameraShake`
  ;[1 1 1] Camera shake
  (`GameplayStatics.PlayWorldCameraShake` "/Script/Engine.CameraShake" (`self.K2_GetActorLocation`) 0.0 500.0))

(fn `UserConstructionScript`
  (`SceneComponent.K2_SetRelativeLocation` (`self.PlayerSpawnPoint`) (`self.PlayerSpawnLocation`) false false)
  (`SceneComponent.K2_SetRelativeLocation` (`self.EnemySpawnPoint`) (`self.EnemySpawnLocation`) false false)
  (`SceneComponent.K2_SetRelativeLocation` (`self.Trigger`) (`self.TriggerLocation`) false false))